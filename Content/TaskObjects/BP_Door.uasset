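; BP_Door is an interactable door that swings open and closed, replicated across the network.
; Interaction goes through InteractOnServer to flip the RepNotify variable InteractRep, whose OnRep calls AnimateOpen.
; A timeline rotates the Arrow component's yaw a quarter turn to open and reverses to close.
; Focus toggles custom depth rendering on the Door, and debug text is hidden at BeginPlay.
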(event `self.ReceiveBeginPlay`
  (`SceneComponent.SetHiddenInGame` (`self.DebugText`) true false))

(event `AnimateOpen`
  (params (Open :type Boolean))
  (if Open
    (bind (_direction _doorfloat) (`Timeline|OpenDoorTimeline` :!via `PlayFromStart` :!label _label)
      (:`Update`
        (`SceneComponent.K2_SetRelativeRotation` (`self.Arrow`) (`KismetMathLibrary.MakeRotator` 0.0 0.0 (`KismetMathLibrary.Lerp` 0.0 -90.0 _doorfloat)) false false)))
    (else
      (goto _label :!via `Reverse`))))

(event `/Game/Interaction/BI_Interaction.Interface_ToggleFocus`
  (params (Focus :type Boolean))
  (`PrimitiveComponent.SetRenderCustomDepth` (`self.Door`) Focus))

(event `/Game/Interaction/BI_Interaction.InterfaceInteract`
  (`self.InteractOnServer`))

(event `InteractOnServer`
  (set `self.InteractRep` (not (`self.InteractRep`))))

(fn `OnRep_InteractRep`
  (`self.AnimateOpen` (`self.InteractRep`)))

(fn `UserConstructionScript`)